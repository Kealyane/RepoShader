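; BP_stool is a wooden stool actor that plays a dissolve effect when anything overlaps its Box, then destroys itself.
; BeginPlay puts a dynamic material instance on the mesh with the effect switched off.
; Overlap switches it on, sets a wood step value and plays a Timeline that feeds elapsed time to the material until it finishes.
; GetEffectTriggerValue exposes the current trigger parameter.
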(event `self.ReceiveBeginPlay`
  (bind _returnvalue (`KismetMaterialLibrary.CreateDynamicMaterialInstance` (`PrimitiveComponent.GetMaterial` (`self.wooden_stool_02_4k`) 0)))
  (bind _output_get (set `self.DynamicMaterial` _returnvalue))
  (`PrimitiveComponent.SetMaterial` (`self.wooden_stool_02_4k`) 0 _output_get)
  (`MaterialInstanceDynamic.SetScalarParameterValue` (`self.DynamicMaterial`) (`self.EffectTriggerParam`) 0.0))

(event `self.Box.OnComponentBeginOverlap`
  (params (OverlappedComponent :type "PrimitiveComponent Object Reference") (OtherActor :type "Actor Object Reference") (OtherComp :type "PrimitiveComponent Object Reference") (OtherBodyIndex :type Integer) (bFromSweep :type Boolean) (SweepResult :type "HitResult Structure (by ref)"))
  (`MaterialInstanceDynamic.SetScalarParameterValue` (`self.DynamicMaterial`) (`self.EffectTriggerParam`) 1.0)
  (`MaterialInstanceDynamic.SetScalarParameterValue` (`self.DynamicMaterial`) (`self.WoodStepParam`) -0.15)
  (bind (_direction _time) (`Timeline|DissolveTimeline`)
    (:`Update`
      (`MaterialInstanceDynamic.SetScalarParameterValue` (`self.DynamicMaterial`) (`self.TimeParam`) _time))
    (:`Finished`
      (`self.K2_DestroyActor`))))

(fn `GetEffectTriggerValue`
  (returns (ReturnValue :type "Float (single-precision)"))
  (bind _returnvalue (`MaterialInstanceDynamic.K2_GetScalarParameterValue` (`self.DynamicMaterial`) (`self.EffectTriggerParam`)))
  (return _returnvalue))

(fn `UserConstructionScript`)